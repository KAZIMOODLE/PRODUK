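; Map actor that builds grids of Case tile actors on BeginPlay, apparently as a movement board.
; Arrays sized to ListMesh define each grid's counts and spacing, though Transform is emptied before being read for placement.
; Each spawned tile gets its per-grid index and is stored in LIStCASE and Dictio.
; The construction-script mesh grid, SpawnCase calls and Manhattan-distance move highlighting are disconnected leftovers that never run.
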(event `self.ReceiveBeginPlay`
  (bind _num (`self.Num`))
  (bind _returnvalue (`KismetArrayLibrary.Array_Length` (`self.ListMesh`)))
  ;[0.1401 1 0] Structure_resize array
  (`KismetArrayLibrary.Array_Resize` _num _returnvalue)
  (`KismetArrayLibrary.Array_Resize` (`self.Space_X`) _returnvalue)
  (`KismetArrayLibrary.Array_Resize` (`self.Space_Y`) _returnvalue)
  (`KismetArrayLibrary.Array_Resize` (`self.NumX`) _returnvalue)
  (`KismetArrayLibrary.Array_Resize` (`self.NumY`) _returnvalue)
  (`KismetArrayLibrary.Array_Resize` (`self.Transform`))
  (for (_ _array_index) _num
    (bind _output (`|GetArrayItem` (`self.NumY`) _array_index))
    (for _index (range (* (`|GetArrayItem` (`self.NumX`) _array_index) _output))
      (bind (_output_location _output_rotation _output_scale) (`KismetMathLibrary.BreakTransform` (`|GetArrayItem` (`self.Transform`) _array_index)))
      (bind _returnvalue_2 (`|SpawnActorFromClass` "/Game/MYSHIzzle/BPS/case.case_C" (`KismetMathLibrary.MakeTransform` (+ _output_location (`KismetMathLibrary.MakeVector` (* (/ _index _output) (`|GetArrayItem` (`self.Space_X`) _array_index)) (* (mod _index _output) (`|GetArrayItem` (`self.Space_Y`) _array_index)))) _output_rotation _output_scale) "Undefined" "OverrideRootScale" null null))
      (`KismetArrayLibrary.Array_Add` (`self.LISt_CASE`) _returnvalue_2)
      (bind _ascase (cast `/Game/MYSHIzzle/BPS/case` _returnvalue_2))
      (bind _output_get (set `/Game/MYSHIzzle/BPS/case.Index` _index _ascase))
      (`BlueprintMapLibrary.Map_Add` (`self.dictio`) _output_get _returnvalue_2))))

(fn `Check Movable Nhighlight`
  (params (casesakchu :type "PrimitiveComponent Object Reference")))

(fn `spawn Case`
  ;[0.1401 1 0] Structure_resize array
  (for (_ _array_index) (`self.Num`)
    (bind _output (`|GetArrayItem` (`self.NumY`) _array_index))
    (for _index (range (* (`|GetArrayItem` (`self.NumX`) _array_index) _output))
      (bind (_output_location _output_rotation _output_scale) (`KismetMathLibrary.BreakTransform` (`|GetArrayItem` (`self.Transform`) _array_index)))
      (`|SpawnActorFromClass` "/Game/MYSHIzzle/BPS/case1.case1_C" (`KismetMathLibrary.ConvertTransformToRelative` (`KismetMathLibrary.MakeTransform` (+ _output_location (`KismetMathLibrary.MakeVector` (* (/ _index _output) (`|GetArrayItem` (`self.Space_X`) _array_index)) (* (mod _index _output) (`|GetArrayItem` (`self.Space_Y`) _array_index)))) _output_rotation _output_scale) (`KismetMathLibrary.MakeTransform` (`SceneComponent.K2_GetComponentLocation` (`self.DefaultSceneRoot`)))) "AlwaysSpawn" "OverrideRootScale" null null))))

(fn `UserConstructionScript`
  ;[0.1401 1 0] Structure_resize array
)